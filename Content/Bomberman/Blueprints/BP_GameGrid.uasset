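; Bomberman level grid actor that lays out a square arena of unbreakable and breakable blocks in its construction script.
; A flat integer array holds each cell type: pillars at odd row and column intersections, then breakables in empty cells, randomly thinned.
; The first and last cells become spawn markers, with nearby array indices cleared.
; Child actor components are then added for both block types; spawn markers get none.
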(event `self.ReceiveBeginPlay`)

(fn `SetBreakables`
  (bind _destructablesamount (`self.DestructablesAmount`))
  (bind _ongridlocation (`self.onGridLocation`))
  (for (_array_element _array_index) _ongridlocation
    (if (== _array_element 0)
      (`KismetArrayLibrary.Array_Set` _ongridlocation _array_index 2)))
  (for (_array_element_2 _array_index_2) _ongridlocation
    (if (and (> (`KismetMathLibrary.RandomInteger` (* _destructablesamount _destructablesamount)) _destructablesamount) (== _array_element_2 2))
      (`KismetArrayLibrary.Array_Set` _ongridlocation _array_index_2))))

(fn `SetSpawnPoints`
  (bind _ongridlocation (`self.onGridLocation`))
  (bind _ongridlocation_2 (`self.onGridLocation`))
  (bind _ongridlocation_3 (`self.onGridLocation`))
  (bind _returnvalue (`KismetArrayLibrary.Array_Length` _ongridlocation))
  (for (_ _array_index) (`self.onGridLocation`)
    (if (== _array_index 0)
      (`KismetArrayLibrary.Array_Set` _ongridlocation_3 _array_index 3)
      (elif (< _array_index 4)
        (`KismetArrayLibrary.Array_Set` _ongridlocation_3 _array_index))))
  (bind _arrayindex (`/Engine/EditorBlueprintResources/StandardMacros.ReverseForEachLoop` _ongridlocation)
    (:`LoopBody`
      (if (== (- _returnvalue 1) _arrayindex)
        (`KismetArrayLibrary.Array_Set` _ongridlocation_2 _arrayindex 3)
        (elif (>= _arrayindex (- _returnvalue 4))
          (`KismetArrayLibrary.Array_Set` _ongridlocation_2 _arrayindex))))))

(fn `SetUnbracables`
  (bind _griddimensions (`self.GridDimensions`))
  (`KismetArrayLibrary.Array_Resize` (`self.onGridLocation`) (* _griddimensions _griddimensions))
  (bind _output_get (set `self.iSize` 1))
  (if (>= _output_get (- (`self.GridDimensions`) 1)) :!label _label
    (return)
    (else
      (set `self.jSize` 1)
      (`KismetArrayLibrary.Array_Set` (`self.onGridLocation`) (+ (* (`self.iSize`) (`self.GridDimensions`)) (`self.jSize`)) 1 :!label _label_2)
      (set `self.jSize` (+ (`self.jSize`) 2))
      (if (>= (`self.jSize`) (- (`self.GridDimensions`) 1))
        (set `self.iSize` (+ (`self.iSize`) 2))
        (goto _label)
        (else
          (goto _label_2))))))

(fn `UserConstructionScript`
  (bind _griddimensions (`self.GridDimensions`))
  (`self.SetUnbracables`)
  (`self.SetBreakables`)
  (`self.SetSpawnPoints`)
  (for _index (range (* _griddimensions _griddimensions))
    (switch `int` (`|GetArrayItem` (`self.onGridLocation`) _index)
      (:`1`
        (bind _returnvalue (`self.GridSizeToLocation` _index))
        (`AddComponent|NODE_AddChildActorComponent-0` :`RelativeTransform` _returnvalue))
      (:`2`
        (`AddComponent|NODE_AddChildActorComponent-1` :`RelativeTransform` _returnvalue)))))