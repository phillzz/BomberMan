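; Shared two-player camera that follows the midpoint between both characters and zooms its spring arm with their distance, within limits.
; On BeginPlay it fades in, blends player controllers' view to itself, finds both characters and starts a looping update timer.
; If either character becomes invalid, the update reruns that setup.
; PlayShake drives a custom timeline shake that adds random offsets to the camera's world location.
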(event `UPDCam`
  (bind _p1 (`self.P1`))
  (bind _p2 (`self.P2`))
  (if (and (`KismetSystemLibrary.IsValid` _p2) (`KismetSystemLibrary.IsValid` _p1))
    (set `SpringArmComponent.TargetArmLength` (`KismetMathLibrary.FClamp` (`self.GetDistanceTo` _p1 _p2) 1000.0 3000.0) (`self.SpringArm`))
    (bind _output_get (set `self.TargetPos` (/ (+ (`self.K2_GetActorLocation` (`self.P1`)) (`self.K2_GetActorLocation` (`self.P2`))) 2.0)))
    (`self.K2_SetActorLocation` (`KismetMathLibrary.VInterpTo` (`self.LastPos`) _output_get (`GameplayStatics.GetWorldDeltaSeconds`) 10.0))
    (set `self.LastPos` (`self.K2_GetActorLocation`))
    (else
      (`PlayerCameraManager.StartCameraFade` :`self` (`GameplayStatics.GetPlayerCameraManager` 0) :`FromAlpha` 1.0 :`Duration` 3.0 :`bShouldFadeAudio` true :!label _label)
      (`KismetSystemLibrary.Delay` 0.1)
      (bind _outactors (`GameplayStatics.GetAllActorsOfClass` "/Script/Engine.PlayerController"))
      (`PlayerController.SetViewTargetWithBlend` _outactors self 2.0 "VTBlend_Linear" 3.0 false)
      (bind _outactors_2 (`GameplayStatics.GetAllActorsOfClass` "/Game/Bomberman/Blueprints/TopDownCharacter.TopDownCharacter_C"))
      (bind _outactors_3 (`GameplayStatics.GetAllActorsOfClass` "/Game/Bomberman/Blueprints/TopDownCharacter2.TopDownCharacter2_C"))
      (set `self.P1` (`|GetArrayItem` _outactors_2))
      (set `self.P2` (`|GetArrayItem` _outactors_3))
      (`KismetSystemLibrary.K2_SetTimer` null "UPDCam" 0.01 true))))

(event `self.ReceiveBeginPlay`
  (goto _label))

(event `PlayShake`
  (bind _returnvalue (`KismetMathLibrary.RandomIntegerInRange` -20 20))
  (bind _returnvalue_2 (`KismetMathLibrary.RandomIntegerInRange` -10 10))
  (bind _returnvalue_3 (`KismetMathLibrary.RandomIntegerInRange` -10 10))
  (bind _camera (`self.Camera`))
  (bind (_returnvalue_x _returnvalue_y _returnvalue_z) (`KismetMathLibrary.BreakVector` (`SceneComponent.K2_GetComponentLocation` _camera)))
  ;[1 1 1] CustomCameraShake
  (bind (_direction _shake) (`Timeline|Shake` :!via `PlayFromStart`)
    (:`Update`
      (`SceneComponent.K2_SetWorldLocation` _camera (`KismetMathLibrary.MakeVector` (+ (* _shake (`KismetMathLibrary.Conv_IntToDouble` (`KismetMathLibrary.Or_IntInt` (`KismetMathLibrary.Clamp` _returnvalue_3 -5 -10) (`KismetMathLibrary.Clamp` _returnvalue_3 5 10)))) _returnvalue_x) (+ (* _shake (`KismetMathLibrary.Conv_IntToDouble` (`KismetMathLibrary.Or_IntInt` (`KismetMathLibrary.Clamp` _returnvalue_2 -5 -10) (`KismetMathLibrary.Clamp` _returnvalue_2 5 10)))) _returnvalue_y) (+ _returnvalue_z (* _shake (`KismetMathLibrary.Conv_IntToDouble` (`KismetMathLibrary.Or_IntInt` (`KismetMathLibrary.Clamp` _returnvalue -10 -20) (`KismetMathLibrary.Clamp` _returnvalue 10 20)))))) false false))))

(fn `UserConstructionScript`)