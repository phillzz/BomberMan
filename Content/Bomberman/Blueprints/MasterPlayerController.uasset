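; Player controller for a Bomberman game that routes second-player input to a second character in the level.
; On BeginPlay it finds and caches the first TopDownCharacter as Player1 and the first TopDownCharacter2 as Player2.
; Player2's move axes and game action are forwarded to that character as message calls after a validity check.
; Player1 is only stored; none of its input is handled here.
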(event `self.ReceiveBeginPlay`
  (bind _outactors (`GameplayStatics.GetAllActorsOfClass` "/Game/TopDownCPP/Blueprints/TopDownCharacter.TopDownCharacter_C"))
  (set `self.Player1` (`|GetArrayItem` _outactors))
  (bind _outactors_2 (`GameplayStatics.GetAllActorsOfClass` "/Game/TopDownCPP/Blueprints/TopDownCharacter2.TopDownCharacter2_C"))
  (set `self.Player2` (`|GetArrayItem` _outactors_2)))

(event `InputAxis|Player2(MoveForward)`
  (params (AxisValue :type "Float (single-precision)"))
  (bind _player2 (`self.Player2`))
  (if (`KismetSystemLibrary.IsValid` _player2)
    (message `/Game/Bomberman/Blueprints/Interaction.CallMoveForward` _player2 AxisValue)))

(event `InputAxis|player2(MoveRight)`
  (params (AxisValue :type "Float (single-precision)"))
  (bind _player2 (`self.Player2`))
  (if (`KismetSystemLibrary.IsValid` _player2)
    (message `/Game/Bomberman/Blueprints/Interaction.CallMoveRight` _player2 AxisValue)))

(event `InputAction|Player2(GameAction)`
  (params (Key :type "Key Structure"))
  (bind _player2 (`self.Player2`))
  (:`Pressed`
    (if (`KismetSystemLibrary.IsValid` _player2)
      (message `/Game/Bomberman/Blueprints/Interaction.CallGameAction` _player2))))

(fn `UserConstructionScript`)