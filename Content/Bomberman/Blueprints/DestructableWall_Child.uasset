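; Destructible wall variant for a Bomberman game that can drop a remote-control item when destroyed.
; DestroyVictim has a one-in-four chance to spawn BP_RemoteControll at the wall's location, then plays an explosion particle and destroys the actor.
; A random Select over four power-up classes is left unconnected, so the remote control is the only possible drop here.
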(event `/Game/Bomberman/Blueprints/Interaction.DestroyVictim`
  (bind _returnvalue (`SceneComponent.K2_GetComponentLocation` (`self.DefaultSceneRoot`)))
  (if (== (`KismetMathLibrary.RandomIntegerInRange` 0 3) 3)
    (`|SpawnActorFromClass` "/Game/Bomberman/Blueprints/BP_RemoteControll.BP_RemoteControll_C" (`KismetMathLibrary.MakeTransform` _returnvalue) "Undefined" "OverrideRootScale" null null))
  (`GameplayStatics.SpawnEmitterAtLocation` "/Game/StarterContent/Particles/P_Explosion.P_Explosion" _returnvalue)
  (`self.K2_DestroyActor`))

(fn `UserConstructionScript`
  (`parent.UserConstructionScript`))