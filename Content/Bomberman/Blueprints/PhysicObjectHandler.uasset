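; Component in the Bomberman game that gives its owning StaticMeshActor a delayed physics drop with effects.
; On BeginPlay it hides the mesh with physics off, then after a short delay reveals it and turns physics simulation on.
; The reveal spawns a steam particle burst and plays a brick-scrape sound at the actor's location, then deactivates the emitter moments later.
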(event `self.ReceiveBeginPlay`
  (bind _returnvalue (`self.GetOwner`))
  (bind _returnvalue_2 (`Actor.K2_GetActorLocation` _returnvalue))
  (bind _asstatic_mesh_actor (cast `StaticMeshActor` _returnvalue))
  (bind _staticmeshcomponent (`StaticMeshActor.StaticMeshComponent` _asstatic_mesh_actor))
  (`PrimitiveComponent.SetSimulatePhysics` _staticmeshcomponent false)
  (`SceneComponent.SetVisibility` (`StaticMeshActor.StaticMeshComponent` _asstatic_mesh_actor) false false)
  (`KismetSystemLibrary.Delay` 2.0)
  (`SceneComponent.SetVisibility` _staticmeshcomponent true false)
  (bind _returnvalue_3 (`GameplayStatics.SpawnEmitterAtLocation` "/Game/StarterContent/Particles/P_Steam_Lit.P_Steam_Lit" _returnvalue_2 (struct) (0.5 0.5 0.5)))
  (`GameplayStatics.PlaySoundAtLocation` "/Game/Bomberman/Audio/77112__benboncan__brick-scrape-4.77112__benboncan__brick-scrape-4" _returnvalue_2)
  (`PrimitiveComponent.SetSimulatePhysics` _staticmeshcomponent true)
  (`KismetSystemLibrary.Delay` 0.1)
  (`self.Deactivate` _returnvalue_3))