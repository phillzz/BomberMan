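; BP_Grid is the Bomberman level grid, generating the block layout in its construction script.
; SetUnbracables marks interior cells at odd row and column indices as unbreakable pillars in the flat OnGridLocation array.
; SetBreakables fills empty cells with breakables, then randomly clears some based on DestructablesDensity.
; Each marked cell becomes a child actor component positioned via Grid2Transform, which maps index to grid position.
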(event `self.ReceiveBeginPlay`)

(event `self.ReceiveTick`
  (params (DeltaSeconds :type "Float (single-precision)")))

(fn `SetBreakables`
  (bind _ongridlocation (`self.onGridLocation`))
  (bind _destructablesdensity (`self.DestructablesDensity`))
  (for (_array_element _array_index) _ongridlocation
    (if (== _array_element 0)
      (`KismetArrayLibrary.Array_Set` _ongridlocation _array_index 2)))
  (for (_array_element_2 _array_index_2) _ongridlocation
    (if (and (> (`KismetMathLibrary.RandomInteger` (* _destructablesdensity (`self.DestructablesDensity`))) _destructablesdensity) (== _array_element_2 2))
      (`KismetArrayLibrary.Array_Set` _ongridlocation _array_index_2)))
  (return))

(fn `SetUnbracables`
  (bind _gridsize (`self.gridSize`))
  (`KismetArrayLibrary.Array_Resize` (`self.onGridLocation`) (* _gridsize _gridsize))
  (bind _output_get (set `self.i` 1))
  (if (>= _output_get (- (`self.gridSize`) 1)) :!label _label
    (return)
    (else
      (set `self.j` 1)
      (`KismetArrayLibrary.Array_Set` (`self.onGridLocation`) (+ (* (`self.i`) (`self.gridSize`)) (`self.j`)) 1 :!label _label_2)
      (set `self.j` (+ (`self.j`) 2))
      (if (>= (`self.j`) (- (`self.gridSize`) 1))
        (set `self.i` (+ (`self.i`) 2))
        (goto _label)
        (else
          (goto _label_2))))))

(fn `UserConstructionScript`
  (locals (x :type Integer) (y :type Integer))
  (bind _gridsize (`self.gridSize`))
  (`self.SetUnbracables`)
  (`self.SetBreakables`)
  (for _index (range (* _gridsize _gridsize))
    (switch `int` (`|GetArrayItem` (`self.onGridLocation`) _index)
      (:`1`
        (bind _returnvalue (`self.Grid2Transform` _index))
        (`AddComponent|NODE_AddChildActorComponent-16` :`RelativeTransform` _returnvalue))
      (:`2`
        (`AddComponent|NODE_AddChildActorComponent-17` :`RelativeTransform` _returnvalue)))))