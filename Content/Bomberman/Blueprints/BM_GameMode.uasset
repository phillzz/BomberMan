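; Bomberman game mode that sets up local multiplayer characters when play begins.
; On BeginPlay it finds every PlayerStart and creates a local player for each one, using the array index as the controller ID.
; The first two indices spawn TopDownCharacter and TopDownCharacter1 at their start transforms, each possessed by the matching player controller.
; Any further starts create a player but spawn no character.
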(event `self.ReceiveBeginPlay`
  (bind _outactors (`GameplayStatics.GetAllActorsOfClass` "/Script/Engine.PlayerStart"))
  (for (_array_element _array_index) _outactors
    (`GameplayStatics.CreatePlayer` _array_index)
    (switch `int` _array_index
      (:`0`
        (bind _returnvalue (`self.GetTransform` _array_element))
        (bind _returnvalue_2 (`|SpawnActorFromClass` "/Game/TopDownCPP/Blueprints/TopDownCharacter.TopDownCharacter_C" _returnvalue "AlwaysSpawn" "OverrideRootScale" null null))
        (`Controller.Possess` (`GameplayStatics.GetPlayerController` _array_index) _returnvalue_2))
      (:`1`
        (bind _returnvalue_3 (`|SpawnActorFromClass` "/Game/TopDownCPP/Blueprints/TopDownCharacter1.TopDownCharacter1_C" _returnvalue "AlwaysSpawn" "OverrideRootScale" null null))
        (`Controller.Possess` (`GameplayStatics.GetPlayerController` _array_index) _returnvalue_3)))))

(fn `UserConstructionScript`)