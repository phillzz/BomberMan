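; Game instance for a Bomberman game that keeps a running tally of match results across levels.
; GameOver takes a win state and increments the draw, Player 1 or Player 2 counter.
; A DoOnce gate counts only the first GameOver call until Reset reopens it.
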(event `/Game/Bomberman/Blueprints/Interaction.GameOver`
  (params (`Win State` :type Integer))
  (`/Engine/EditorBlueprintResources/StandardMacros.DoOnce` false :!label _label
    (:`Completed`
      (switch `int` `Win State`
        (:`0`
          (set `self.Draws` (+ (`self.Draws`) 1)))
        (:`1`
          (set `self.Player1` (+ (`self.Player1`) 1)))
        (:`2`
          (set `self.Player2` (+ (`self.Player2`) 1)))))))

(event `Reset`
  (goto _label :!via `Reset`))